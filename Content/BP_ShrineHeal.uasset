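; BP_ShrineHeal is a healing shrine Blueprint that handles the visual and audio feedback, with no healing logic in its graphs.
; UpdateVisuals swaps the mesh between green and red debug materials to show availability.
; TriggerHealEffects attaches a particle emitter to the Techo component, then destroys it after a fixed delay.
; Placeholder sounds mark the effect's start and end, both played at world origin rather than at the shrine.
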(event `self.UpdateVisuals`
  (params (bAvailable :type Boolean))
  (bind _meshcomp (`self.MeshComp`))
  (if bAvailable
    (`PrimitiveComponent.SetMaterial` _meshcomp 0 "/Engine/EngineDebugMaterials/VertexColorViewMode_GreenOnly.VertexColorViewMode_GreenOnly")
    (else
      (`PrimitiveComponent.SetMaterial` _meshcomp 0 "/Engine/EngineDebugMaterials/VertexColorViewMode_RedOnly.VertexColorViewMode_RedOnly"))))

(event `self.TriggerHealEffects`
  (bind _returnvalue (`GameplayStatics.SpawnEmitterAttached` "/Engine/Tutorial/SubEditors/TutorialAssets/TutorialParticleSystem.TutorialParticleSystem" (`self.Techo`)))
  (`GameplayStatics.PlaySoundAtLocation` "/Engine/VREditor/Sounds/UI/Camera_Shutter.Camera_Shutter" (0.0 0.0 0.0) (struct) 1.0 1.0 0.0 null null null null)
  (`KismetSystemLibrary.Delay` 5.0)
  (`ActorComponent.K2_DestroyComponent` _returnvalue)
  (`GameplayStatics.PlaySoundAtLocation` "/Engine/VREditor/Sounds/UI/Foliage_Placed.Foliage_Placed" (0.0 0.0 0.0) (struct) 1.0 1.0 0.0 null null null null))

(fn `UserConstructionScript`)